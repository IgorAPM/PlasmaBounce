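; Base projectile actor that deals damage to the actors it hits, other than its own instigator.
; Fire activates the ProjectileMovement component and sets a local-space velocity from speed and direction, while Disable deactivates it.
; Sphere hits apply BaseDamage with the projectile as causer, then cast to BP_BaseEnemy, which so far only triggers a debug print.
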(event `self.ReceiveBeginPlay`)

(event `self.ReceiveTick`
  (params (DeltaSeconds :type "Float (single-precision)")))

(event `Fire`
  (params (Speed :type "Float (double-precision)" :default 1000.0) (Direction :type "Vector Structure"))
  (bind _projectilemovement (`self.ProjectileMovement`))
  (`ActorComponent.Activate` _projectilemovement true)
  (`ProjectileMovementComponent.SetVelocityInLocalSpace` _projectilemovement (* Speed Direction)))

(event `Disable`
  (`ActorComponent.Deactivate` (`self.ProjectileMovement`)))

(event `self.Sphere.OnComponentHit`
  (params (HitComponent :type "PrimitiveComponent Object Reference") (OtherActor :type "Actor Object Reference") (OtherComp :type "PrimitiveComponent Object Reference") (NormalImpulse :type "Vector Structure") (Hit :type "HitResult Structure (by ref)"))
  (if (!= OtherActor (`self.GetInstigator`))
    (`GameplayStatics.ApplyDamage` OtherActor (`self.Base Damage`) null self)
    (cast `/Game/PlasmaBounce/Blueprints/Pawns/BP_BaseEnemy` OtherActor)
    (`KismetSystemLibrary.PrintString` "Hello")))

(fn `UserConstructionScript`)