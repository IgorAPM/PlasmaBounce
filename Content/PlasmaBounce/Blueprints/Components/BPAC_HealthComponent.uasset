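; BPAC_HealthComponent is a health component that tracks damage and death for its owner.
; Health starts at MaxHealth on BeginPlay, and HandleDamage subtracts incoming damage.
; Non-lethal hits broadcast OnDamageTaken with current and maximum health.
; Lethal hits broadcast OnDeath through a DoOnce so it fires only once, leaving Health at its last value.
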(event `self.ReceiveBeginPlay`
  (set `self.Health` (`self.MaxHealth`)))

(event `HandleDamage`
  (params (Damage :type "Float (double-precision)"))
  (bind _returnvalue (- (`self.Health`) Damage))
  (if (<= _returnvalue 0.0)
    (`/Engine/EditorBlueprintResources/StandardMacros.DoOnce` false
      (:`Completed`
        (`self.OnDeath`)))
    (else
      (bind _output_get (set `self.Health` _returnvalue))
      (`self.OnDamageTaken` _output_get (`self.MaxHealth`)))))