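; Base player pawn that aims by yaw while Aim/Shoot is held and fires a timed volley of projectiles on release.
; Tick clamps yaw to a forward arc, and the mouse cursor stays visible.
; Fire reuses projectiles from a pool by index, spawning and adding any that are missing.
; The level's BP_ProjectileCollector reports returns, which are hidden and disabled, re-enabling firing once the whole volley is collected.
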(event `self.ReceiveBeginPlay`
  (bind _returnvalue (`GameplayStatics.GetPlayerController` 0))
  (`WidgetBlueprintLibrary.SetInputMode_GameAndUIEx` _returnvalue null "DoNotLock" false)
  (set `PlayerController.bShowMouseCursor` true _returnvalue)
  (bind _returnvalue_2 (`GameplayStatics.GetActorOfClass` "/Game/PlasmaBounce/Blueprints/Actors/BP_ProjectileCollector.BP_ProjectileCollector_C"))
  (bind _output_get (set `self.ProjectileCollector` _returnvalue_2))
  (add `/Game/PlasmaBounce/Blueprints/Actors/BP_ProjectileCollector.OnProjectileCollected` _output_get (delegate `OnProjectileCollected`)))

(event `OnProjectileCollected`
  (params (Projectile :type "/Game/PlasmaBounce/Blueprints/Actors/BP_BaseProjectile Object Reference"))
  (`self.ResetProjectile` Projectile)
  (if (>= (`/Game/PlasmaBounce/Blueprints/Actors/BP_ProjectileCollector.CollectedProjectiles` (`self.ProjectileCollector`)) (`self.ProjectileCount`))
    (set `self.bCanFire` true)))

(event `self.ReceiveTick`
  (params (DeltaSeconds :type "Float (single-precision)"))
  (bind (_returnvalue_roll _returnvalue_pitch _returnvalue_yaw) (`KismetMathLibrary.BreakRotator` (`self.K2_GetActorRotation`)))
  (`self.K2_SetActorRotation` (`KismetMathLibrary.MakeRotator` _returnvalue_roll _returnvalue_pitch (`KismetMathLibrary.FClamp` _returnvalue_yaw -80.0 80.0))))

(event `InputAction|Aim/Shoot`
  (params (Key :type "Key Structure"))
  (:`Pressed`
    (set `self.IsAiming` true))
  (:`Released`
    (set `self.IsAiming` false)
    (if (`self.bCanFire`)
      (`self.Fire`))))

(event `InputAxis|Turn`
  (params (AxisValue :type "Float (single-precision)"))
  (if (and (`self.IsAiming`) (`self.bCanFire`))
    (`self.AddControllerYawInput` AxisValue)))

(event `Fire`
  (set `self.bCanFire` false)
  (set `/Game/PlasmaBounce/Blueprints/Actors/BP_ProjectileCollector.CollectedProjectiles` 0 (`self.ProjectileCollector`))
  (bind _index (`/Game/PlasmaBounce/Blueprints/Libraries/ML_CustomMacros.ForLoopWithDelay` 0 (- (`self.ProjectileCount`) 1) 0.2)
    (:`LoopBody`
      (bind _output (`|GetArrayItem` (`self.ProjectilePool`) _index))
      (`/Engine/EditorBlueprintResources/StandardMacros.IsValid` _output
        (:`Is Valid`
          (`self.SetActorHiddenInGame` _output false)
          (`self.K2_SetActorTransform` _output (`SceneComponent.K2_GetComponentToWorld` (`self.ProjectileSpawner`)) false true)
          (`/Game/PlasmaBounce/Blueprints/Actors/BP_BaseProjectile.Fire` _output 1000.0 (1.0 0.0 0.0)))
        (:`Is Not Valid`
          (bind _returnvalue (`|SpawnActorFromClass` "/Game/PlasmaBounce/Blueprints/Actors/BP_BaseProjectile.BP_BaseProjectile_C" (`SceneComponent.K2_GetComponentToWorld` (`self.ProjectileSpawner`)) "Undefined" "OverrideRootScale" self self))
          (`/Game/PlasmaBounce/Blueprints/Actors/BP_BaseProjectile.Fire` _returnvalue 1000.0 (1.0 0.0 0.0))
          (`KismetArrayLibrary.Array_Add` (`self.ProjectilePool`) _returnvalue))))))

(event `ResetProjectile`
  (params (Projectile :type "/Game/PlasmaBounce/Blueprints/Actors/BP_BaseProjectile Object Reference"))
  (`self.SetActorHiddenInGame` Projectile true)
  (`/Game/PlasmaBounce/Blueprints/Actors/BP_BaseProjectile.Disable` Projectile))

(fn `UserConstructionScript`)