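; Player character Blueprint that fires a pool of projectiles and tracks their return through a BP_ProjectileCollector.
; On BeginPlay it finds the collector and binds its collected event, disabling each collected projectile and setting CanFire once the count reaches ProjectileCount.
; FireAllProjectiles resets that count, then uses a delayed loop to teleport each pooled projectile to ShotRoot and launch it along +X at RateOfFire intervals.
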(event `self.ReceiveBeginPlay`
  (bind _returnvalue (`GameplayStatics.GetActorOfClass` "/Game/PlasmaBounce/Blueprints/Actors/BP_ProjectileCollector.BP_ProjectileCollector_C"))
  (bind _output_get (set `self.ProjectileCollector` _returnvalue))
  (add `/Game/PlasmaBounce/Blueprints/Actors/BP_ProjectileCollector.OnProjectileCollected` _output_get (delegate `CollectProjectile`)))

(event `CollectProjectile`
  (params (Projectile :type "BaseProjectile Object Reference"))
  (`BaseProjectile.Disable` Projectile)
  (if (>= (`/Game/PlasmaBounce/Blueprints/Actors/BP_ProjectileCollector.CollectedProjectiles` (`self.ProjectileCollector`)) (`self.ProjectileCount`))
    (set `self.bCanFire` true)))

(event `self.FireAllProjectiles`
  (set `/Game/PlasmaBounce/Blueprints/Actors/BP_ProjectileCollector.CollectedProjectiles` 0 (`self.ProjectileCollector`))
  (bind _array_element (`/Game/PlasmaBounce/Blueprints/Libraries/ML_CustomMacros.ForEachLoopWithDelay` (`self.ProjectilePool`) (`self.RateOfFire`))
    (:`LoopBody`
      (`self.K2_SetActorTransform` _array_element (`SceneComponent.K2_GetComponentToWorld` (`self.ShotRoot`)) false true)
      (`BaseProjectile.OnFired` _array_element (1.0 0.0 0.0) 1000.0))))

(fn `UserConstructionScript`)