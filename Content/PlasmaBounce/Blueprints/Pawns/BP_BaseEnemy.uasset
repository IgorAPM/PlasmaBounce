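; BP_BaseEnemy is the base enemy pawn for PlasmaBounce, giving enemies health, a health bar and death.
; AnyDamage is forwarded to the BPAC_HealthComponent, whose OnDamageTaken event updates the WB_HealthBar inside the Widget component.
; When the health component fires OnDeath, the enemy prints a death message with its name and destroys itself.
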(event `self.ReceiveAnyDamage`
  (params (Damage :type "Float (single-precision)") (DamageType :type "DamageType Object Reference") (InstigatedBy :type "Controller Object Reference") (DamageCauser :type "Actor Object Reference"))
  (`/Game/PlasmaBounce/Blueprints/Components/BPAC_HealthComponent.HandleDamage` (`self.BPAC_HealthComponent`) Damage))

(event `self.BPAC_HealthComponent.OnDeath`
  (`KismetSystemLibrary.PrintString` (`KismetTextLibrary.Conv_TextToString` (`|FormatText` "{name} died." (`KismetSystemLibrary.GetDisplayName` self))))
  (`self.K2_DestroyActor`))

(event `self.BPAC_HealthComponent.OnDamageTaken`
  (params (CurrentHealth :type "Float (double-precision)") (MaxHealth :type "Float (double-precision)"))
  (bind _aswb_health_bar (cast `/Game/PlasmaBounce/Blueprints/UI/WB_HealthBar` (`WidgetComponent.GetWidget` (`self.Widget`))))
  (`/Game/PlasmaBounce/Blueprints/UI/WB_HealthBar.DisplayDamage` _aswb_health_bar CurrentHealth MaxHealth))

(fn `UserConstructionScript`)